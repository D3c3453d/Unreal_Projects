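; BP_God is a manager actor that creates the on-screen UI at BeginPlay and passes it a reference to itself.
; SpawnBullet places a BP_BulletNail at a random navmesh location around the actor and tracks it in the Bullets array.
; GetBullet claims a given bullet by removing it from that array, returning it only if the removal succeeds.
; The event-graph loop that calls SpawnBullet is disconnected and never runs.
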(event EventBeginPlay
  (bind _returnvalue (UserInterface|CreateWidget "/Game/Tanki/Tanks/Tank1/UI.UI_C"))
  (Variables|/Game/Tanki/Tanks/Tank1/UI.UI_C|SetGod _returnvalue self)
  (UserInterface|Viewport|AddtoViewport _returnvalue 0))

(event Collision|EventActorBeginOverlap
  (params (OtherActor :type Actor%20Object%20Reference)))

(event EventTick
  (params (DeltaSeconds :type Float%20%28single-precision%29)))

(fn ConstructionScript)

(fn SpawnBullet
  (bind _randomlocation (Class|NavigationSystemV1|GetRandomLocationinNavigableRadius (Transformation|GetActorLocation self) 1e+03 (Variables|Default|GetNav%20Data) 0))
  (bind _returnvalue (Game|SpawnActorfromClass "/Game/Tanki/Resources/BP_BulletNail.BP_BulletNail_C" (Math|Transform|MakeTransform _randomlocation "0, 0, 0" "1,1,1") "Undefined" 0 0))
  (Utilities|Array|Add (Variables|Default|GetBullets) _returnvalue))

(fn GetBullet
  (params (Bullet :type BP%20Bullet%20Nail%20Object%20Reference))
  (bind _returnvalue (Utilities|Array|RemoveItem (Variables|Default|GetBullets) Bullet))
  (if _returnvalue
    (return Bullet)
    (else
      (return 0))))