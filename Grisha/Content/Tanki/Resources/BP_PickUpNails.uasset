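; BP_PickUpNails is a pickup actor that gives nails to a Tank1 that overlaps it.
; On overlap it casts the other actor to Tank1, destroys itself and adds a fixed amount to that tank's NailAmount.
; A timeline started on BeginPlay animates the pickup, yawing the actor by its track value and setting the Nail component's relative location on each update.
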(event EventBeginPlay
  ;[1 1 1] Rotation
  (bind _newtrack_0 (Timeline|Animation Play)
    (:Update
      (Class|Actor|AddActorWorldRotation (Components|GetOwner (Variables|Default|GetNail)) (Math|Rotator|MakeRotator 0.0 0.0 (* _newtrack_0 5.0)))
      (Transformation|SetRelativeLocation (Variables|Default|GetNail) (Math|Vector|MakeVector 0.0 0.0 0.0) false false))))

(event Collision|EventActorBeginOverlap
  (params (OtherActor :type Actor%20Object%20Reference))
  ;[1 1 1] Pick Up
  (bind _astank_1 (Utilities|Casting|CastToTank1 OtherActor))
  (Actor|DestroyActor)
  (Variables|/Game/Tanki/Tanks/Tank1/Tank1.Tank1_C|SetNailAmount _astank_1 (+ (Variables|/Game/Tanki/Tanks/Tank1/Tank1.Tank1_C|GetNailAmount _astank_1) 10)))

(event EventTick
  (params (DeltaSeconds :type Float%20%28single-precision%29)))

(fn ConstructionScript)